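; BP_Silo is a production silo that simulates a clean-in-place (CIP) cycle on its fluid level.
; RunCIPCleaningCycle chains three stages: flush inventory to empty, fill with cleaning reagent to a target level, then flush again.
; Looping function-name timers step the level by flow rate, each triggering the next stage while updating valve and completion flags.
; An already-empty silo never starts the flush timer, so the cycle stalls.
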(event `TickFlushInventory`
  (bind _fluidlevel (`self.FluidLevel`))
  (set `self.FluidLevel` (- _fluidlevel (* (`self.FlushFlowRate`) 0.2)))
  (if (not (> _fluidlevel 0.0))
    (set `self.FluidLevel` 0.0)
    (`KismetSystemLibrary.K2_ClearTimer` null "TickFlushInventory")
    (set `self.FinishedFlush` true)
    (`self.FillCIP`)))

(event `TickFillCIP`
  (bind _fluidlevel (`self.FluidLevel`))
  (bind _cleaningtargetlevel (`self.CleaningTargetLevel`))
  (set `self.FluidLevel` (+ _fluidlevel (* (`self.CleaningFlowRate`) 0.2)))
  (if (> _fluidlevel _cleaningtargetlevel)
    (set `self.FluidLevel` _cleaningtargetlevel)
    (`KismetSystemLibrary.K2_ClearTimer` null "TickFillCIP")
    (set `self.FinishedCleaningReagent` true)
    (`self.FlushCIP`)))

(event `TickFlushCIP`
  (bind _fluidlevel (`self.FluidLevel`))
  (set `self.FluidLevel` (- _fluidlevel (* (`self.FlushFlowRate`) 0.2)))
  (if (not (> _fluidlevel 0.0))
    (set `self.FluidLevel` 0.0)
    (`KismetSystemLibrary.K2_ClearTimer` null "TickFlushCIP")
    (set `self.FinishedFlushCleaningReagent` true)
    (set `self.RunningCleaningCycle` false)
    (set `self.CleaningInletValve` false)
    (set `self.FlushOutletValve` false)))

(fn `FillCIP`
  (set `self.FlushOutletValve` false)
  (set `self.CleaningInletValve` true)
  (`KismetSystemLibrary.K2_SetTimer` null "TickFillCIP" 0.2 true))

(fn `FlushCIP`
  (set `self.CleaningInletValve` false)
  (set `self.FlushOutletValve` true)
  (`KismetSystemLibrary.K2_SetTimer` null "TickFlushCIP" 0.2 true))

(fn `FlushInventory`
  (if (> (`self.FluidLevel`) 0.0)
    (set `self.FlushOutletValve` true)
    (`KismetSystemLibrary.K2_SetTimer` null "TickFlushInventory" 0.2 true)))

(fn `RunCIPCleaningCycle`
  (set `self.RunningCleaningCycle` true)
  (set `self.FinishedFlush` false)
  (set `self.FinishedCleaningReagent` false)
  (set `self.FinishedFlushCleaningReagent` false)
  (`self.FlushInventory`))

(fn `UserConstructionScript`
  (set `self.FlushOutletValve` false)
  (set `self.CleaningInletValve` false)
  (set `self.RunningCleaningCycle` false)
  (set `self.FlushFlowRate` 10.0)
  (set `self.CleaningTargetLevel` 100.0)
  (set `self.CleaningFlowRate` 10.0)
  (set `self.FinishedFlush` true)
  (set `self.FinishedCleaningReagent` true)
  (set `self.FinishedFlushCleaningReagent` true))