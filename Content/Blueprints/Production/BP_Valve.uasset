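; BP_Valve is an interactable valve that spins and switches between open and closed.
; Interact is ignored while the valve is moving or the level's BP_Emergency_Stop, found on BeginPlay, is triggered.
; Otherwise it alternately plays or reverses the RotateValve timeline, which lerps ShapeCube's yaw through a full turn.
; When the timeline finishes, it clears the moving lock and toggles IsOpen, which starts as closed.
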(event `self.ReceiveBeginPlay`
  (bind _outactors (`GameplayStatics.GetAllActorsOfClass` "/Game/Blueprints/Production/BP_Emergency_Stop.BP_Emergency_Stop_C"))
  (set `self.EmergencyStop` (`|GetArrayItem` _outactors)))

(event `ToggleValve`
  (if (`self.IsOpen`)
    (set `self.IsOpen` false)
    (else
      (set `self.IsOpen` true))))

(event `/Game/Blueprints/InteractionInterface.Interact`
  (if (`/Game/Blueprints/Production/BP_Emergency_Stop.IsTriggered` (`self.EmergencyStop`))
    _
    (elif (not (`self.IsValveMoving?`))
      (set `self.IsValveMoving?` true)
      (bind _output_get (set `self.Rotating?` (not (`self.Rotating?`))))
      (if _output_get
        (bind (_direction _alpha) (`Timeline|RotateValve` :!label _label)
          (:`Update`
            (`SceneComponent.K2_SetRelativeRotation` (`self.Shape_Cube`) (`KismetMathLibrary.MakeRotator` 0.0 0.0 (`KismetMathLibrary.Lerp` 0.0 360.0 _alpha)) false false)
            (set `self.Finished?` true))
          (:`Finished`
            (set `self.IsValveMoving?` false)
            (`self.ToggleValve`)))
        (else
          (goto _label :!via `Reverse`))))))

(fn `UserConstructionScript`
  (set `self.IsOpen` false))