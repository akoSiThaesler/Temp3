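; BP_Reactor is a production reactor that doses two materials to ordered amounts, mixes them and runs a CIP cleaning cycle.
; UpdateFluidLevels accumulates material from flowing pipes, asks DataManager for educt B once A overfills, and starts mixing when both match.
; A timeline spins the blade during a timed mix, after which active orders are deleted and DataManager empties the reactor.
; Cleaning chains looping timers: flush, reagent fill, final flush.
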(event `MixingMaterials`
  (bind _mixerblade (`self.MixerBlade`))
  (set `self.FinishedMixing` false)
  (set `self.MixingTimeLeft` (`self.MixingDuration`))
  (`KismetSystemLibrary.K2_SetTimer` null "UpdateMixingTimer" 1.0 true)
  (bind (_direction _rotation) (`Timeline|MixerRotation` :!label _label)
    (:`Update`
      (`SceneComponent.K2_SetRelativeLocationAndRotation` _mixerblade (`SceneComponent.RelativeLocation` _mixerblade) (`KismetMathLibrary.MakeRotator` 0.0 0.0 _rotation) false false))))

(event `StopMixerRotation`
  (goto _label :!via `Stop`))

(event `TickFlushInventory`
  (bind _fluidlevel (`self.FluidLevel`))
  (set `self.FluidLevel` (- _fluidlevel (* (`self.FlushFlowRate`) 0.2)))
  (if (not (> _fluidlevel 0.0))
    (set `self.FluidLevel` 0.0)
    (`KismetSystemLibrary.K2_ClearTimer` null "TickFlushInventory")
    (set `self.FinishedFlush` true)
    (`self.FillCIP`)))

(event `TickFillCIP`
  (bind _cleaningtargetlevel (`self.CleaningTargetLevel`))
  (bind _fluidlevel (`self.FluidLevel`))
  (set `self.FluidLevel` (+ _fluidlevel (* (`self.InletFlowRate`) 0.2)))
  (if (> _fluidlevel _cleaningtargetlevel)
    (set `self.FluidLevel` _cleaningtargetlevel)
    (`KismetSystemLibrary.K2_ClearTimer` null "TickFillCIP")
    (set `self.FinishedCleaningReagent` true)
    (`self.FlushCIP`)))

(event `TickFlushCIP`
  (bind _fluidlevel (`self.FluidLevel`))
  (set `self.FluidLevel` (- _fluidlevel (* (`self.FlushFlowRate`) 0.2)))
  (if (not (> _fluidlevel 0.0))
    (set `self.FluidLevel` 0.0)
    (`KismetSystemLibrary.K2_ClearTimer` null "TickFlushCIP")
    (set `self.FinishedFlushCleaningReagent` true)
    (set `self.RunningCleaningCycle` false)
    (set `self.FlushOutletValve` false)
    (set `self.CleaningInletValve` false)))

(fn `FillCIP`
  (set `self.FlushOutletValve` false)
  (set `self.CleaningInletValve` true)
  (`KismetSystemLibrary.K2_SetTimer` null "TickFillCIP" 0.2 true))

(fn `FlushCIP`
  (set `self.CleaningInletValve` false)
  (set `self.FlushOutletValve` true)
  (`KismetSystemLibrary.K2_SetTimer` null "TickFlushCIP" 0.2 true))

(fn `FlushInventory`
  (if (> (`self.FluidLevel`) 0.0)
    (set `self.FlushOutletValve` true)
    (`KismetSystemLibrary.K2_SetTimer` null "TickFlushInventory" 0.2 true)))

(fn `RunCIPCleaningCycle`
  (set `self.RunningCleaningCycle` true)
  (set `self.FinishedFlush` false)
  (set `self.FinishedCleaningReagent` false)
  (set `self.FinishedFlushCleaningReagent` false)
  (`self.FlushInventory`))

(fn `UpdateFluidLevels`
  (returns (FluidIn :type "Float (double-precision)"))
  (bind _orderedmaterialb (`self.OrderedMaterialB`))
  (bind _orderedmateriala (`self.OrderedMaterialA`))
  (bind _materiala (`self.MaterialA`))
  (bind _materialb (`self.MaterialB`))
  (for (_array_element _array_index) (`self.ConnectedPipes`)
    (if (== _array_index 0)
      (bind _isflowing (`/Game/Blueprints/Production/Bp_pipe_straight_Silo_Reactor.IsFlowing` _array_element))
      (if _isflowing
        (bind _materialamount (`/Game/Blueprints/Production/Bp_pipe_straight_Silo_Reactor.MaterialAmount` _array_element))
        (bind _returnvalue (+ _materiala _materialamount))
        (if (<= _returnvalue _orderedmateriala)
          (bind _output_get (set `self.MaterialA` _returnvalue))
          (bind _returnvalue_2 (+ _output_get (stale _output_get_2)))
          (set `self.FluidLevel` _returnvalue_2 :!label _label)
          (else
            (`/Game/Blueprints/Production/BP_FacilityDataManager.FillEductB` (`self.DataManager`))
            (set `self.MaterialA` _orderedmateriala)
            (set `/Game/Blueprints/Production/Bp_pipe_straight_Silo_Reactor.IsFlowing` false _array_element :!label _label_2)
            (set `self.FluidLevel` (+ _materiala _orderedmaterialb))
            (for _array_element_2 (`/Game/Blueprints/Production/Bp_pipe_straight_Silo_Reactor.ValveReferences` _array_element)
              (set `/Game/Blueprints/Production/BP_Valve.IsOpen` false _array_element_2)))))
      (elif _isflowing
        (bind _returnvalue_3 (+ _materialamount _materialb))
        (if (<= _returnvalue_3 _orderedmaterialb)
          (bind _output_get_2 (set `self.MaterialB` _returnvalue_3))
          (goto _label)
          (else
            (set `self.MaterialB` _orderedmaterialb)
            (goto _label_2))))))
  (if (== _orderedmateriala _materiala)
    (if (== _materialb _orderedmaterialb)
      (`self.MixingMaterials`)
      (bind _output_get_3 (set `self.FluidLevel` _returnvalue_2))
      (return _output_get_3))))

(fn `UpdateMixingTimer`
  (bind _datamanager (`self.DataManager`))
  (if (not (`self.FinishedMixing`))
    (bind _output_get (set `self.MixingTimeLeft` (- (`self.MixingTimeLeft`) 1.0)))
    (if (<= _output_get 0.0)
      (`self.StopMixerRotation`)
      (`KismetSystemLibrary.K2_ClearTimer` null "UpdateMixingTimer")
      (for _array_element (`/Game/Blueprints/Production/BP_FacilityDataManager.ActiveOrders` _datamanager)
        (if (`.IsActive_9_70044C44437D228BF81974808908D2DF` (break `/Game/Blueprints/Production/STR_Order` _array_element))
          (`/Game/Blueprints/Production/BP_FacilityDataManager.DeleteOrder` _datamanager _array_element)))
      (set `self.FinishedMixing` true)
      (set `self.MaterialA` 0.0)
      (set `self.MaterialB` 0.0)
      (`/Game/Blueprints/Production/BP_FacilityDataManager.EmptyReactor` _datamanager))))

(fn `UserConstructionScript`
  (set `self.MaterialA` 0.0)
  (set `self.MaterialB` 0.0)
  (set `self.MaxCapacity` 10000.0)
  (set `self.FluidLevel` 0.0)
  (set `self.OrderedMaterialA` 200.0)
  (set `self.OrderedMaterialB` 200.0)
  (set `self.MixingDuration` 10.0)
  (set `self.FinishedMixing` true)
  (set `self.FlushOutletValve` false)
  (set `self.CleaningInletValve` false)
  (set `self.RunningCleaningCycle` false)
  (set `self.FlushFlowRate` 10.0)
  (set `self.InletFlowRate` 10.0)
  (set `self.CleaningTargetLevel` 100.0)
  (set `self.FinishedFlush` true)
  (set `self.FinishedCleaningReagent` true)
  (set `self.FinishedFlushCleaningReagent` true))