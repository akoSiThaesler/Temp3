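; Spline-built pipe that moves fluid from a Source to a Target, apparently silo to reactor, through a pump and valves.
; The construction script lays spline mesh sections with rings and spawns BP_Valve child actors along the spline.
; Each tick, flow requires an active pump, all valves open and Target.FinishedMixing, otherwise open valves get closed.
; Flow drains Source by pump rate and updates Target, stopping at empty or full; idle Source levels snap to hundreds.
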(event `self.ReceiveTick`
  (params (DeltaSeconds :type "Float (single-precision)"))
  (`self.VolumeCalculationMain` DeltaSeconds))

(fn `PipeSpline`
  (params (Spline :type "SplineComponent Object Reference") (SectionLength :type "Float (double-precision)") (Index :type Integer))
  (returns (SplineRingPos :type "Vector Structure") (SplineRingRotation :type "Vector Structure"))
  (bind (_splinepipestart _splinepipestartrotation _splinepipeend _splinepipeendrotation _splineringpos _splinerintrotation) (`self.SplineLocationRotation` Spline SectionLength Index))
  (bind _returnvalue (`AddComponent|NODE_AddSplineMeshComponent-0`))
  (`PrimitiveComponent.SetCollisionEnabled` _returnvalue "QueryAndPhysics")
  (`SplineMeshComponent.SetForwardAxis` _returnvalue "X" true)
  (`SplineMeshComponent.SetStartAndEnd` _returnvalue _splinepipestart _splinepipestartrotation _splinepipeend _splinepipeendrotation true)
  (return _splineringpos _splinerintrotation))

(fn `RingSpline`
  (params (Index :type Integer) (Spline :type "SceneComponent Object Reference") (SplineRingPos :type "Vector Structure") (SplineRingRotation :type "Vector Structure (by ref)"))
  (if (`KismetMathLibrary.Conv_IntToBool` (mod Index 3))
    (bind _returnvalue (`AddComponent|NODE_AddStaticMeshComponent-1`))
    (`SceneComponent.K2_SetWorldLocationAndRotation` _returnvalue (+ SplineRingPos (`SceneComponent.K2_GetComponentLocation` Spline)) (`KismetMathLibrary.MakeRotFromX` SplineRingRotation) false false)))

(fn `SplineLength`
  (params (Spline :type "SplineComponent Object Reference") (SectionLength :type "Float (double-precision)"))
  (returns (SplineLength :type "Float (double-precision)"))
  (return (/ (`SplineComponent.GetSplineLength` Spline) SectionLength)))

(fn `SplineLocationRotation`
  (params (Spline :type "SplineComponent Object Reference") (SectionLength :type "Float (double-precision)") (Index :type Integer))
  (returns (SplinePipeStart :type "Vector Structure") (SplinePipeStartRotation :type "Vector Structure") (SplinePipeEnd :type "Vector Structure") (SplinePipeEndRotation :type "Vector Structure") (SplineRingPos :type "Vector Structure") (SplineRintRotation :type "Vector Structure"))
  (bind _returnvalue (* Index SectionLength))
  (bind _returnvalue_2 (`SplineComponent.GetLocationAtDistanceAlongSpline` Spline _returnvalue "Local"))
  (bind _returnvalue_3 (* (+ Index 1) SectionLength))
  (bind _returnvalue_4 (`SplineComponent.GetTangentAtDistanceAlongSpline` Spline _returnvalue_3 "Local"))
  (return (- _returnvalue_2 (0.5 0.0 0.0)) (`KismetMathLibrary.ClampVectorSize` (`SplineComponent.GetTangentAtDistanceAlongSpline` Spline _returnvalue "Local") 0.0 SectionLength) (+ (`SplineComponent.GetLocationAtDistanceAlongSpline` Spline _returnvalue_3 "Local") (0.5 0.0 0.0)) (`KismetMathLibrary.ClampVectorSize` _returnvalue_4 0.0 SectionLength) _returnvalue_2 _returnvalue_4))

(fn `UpdateFlowState`
  (bind _valvereferences (`self.ValveReferences`))
  (bind _source (`self.Source`))
  (bind _target (`self.Target`))
  (bind _maxcapacity (`/Game/Blueprints/Production/BP_Reactor.MaxCapacity` _target))
  (set `self.IsFlowing` false)
  (for _array_element _valvereferences
    (if (`/Game/Blueprints/Production/BP_Valve.IsOpen` _array_element)
      (if (< (`/Game/Blueprints/Production/BP_Silo.FluidLevel` _source) 0.0)
        (set `/Game/Blueprints/Production/BP_Silo.FluidLevel` 0.0 _source)
        (for _array_element_2 _valvereferences :!label _label
          (set `/Game/Blueprints/Production/BP_Valve.IsOpen` true _array_element_2))
        (break)
        (elif (> (`/Game/Blueprints/Production/BP_Reactor.FluidLevel` _target) _maxcapacity)
          (set `/Game/Blueprints/Production/BP_Reactor.FluidLevel` _maxcapacity _target)
          (goto _label)
          (elif (`/Game/Blueprints/Production/BP_Pump.IsActive` (`self.Pump`))
            (set `self.IsFlowing` true)
            (else
              (break)))))
      (else
        (break)))))

(fn `UserConstructionScript`
  (bind _spline (`self.Spline`))
  (bind _sectionlength (`self.SectionLength`))
  (bind _splinelength (`self.SplineLength` _spline _sectionlength))
  (for _index (range (+ (`KismetMathLibrary.FTrunc` _splinelength) 1))
    (bind (_splineringpos _splineringrotation) (`self.PipeSpline` _spline _sectionlength _index))
    (`self.RingSpline` _index _spline _splineringpos _splineringrotation))
  (`self.ValveSpline` _splinelength _spline)
  (`self.UpdateFlowState`))

(fn `ValveSpline`
  (params (SplineLength :type "Float (double-precision)") (Spline :type "SplineComponent Object Reference"))
  (for _array_element (`self.ValvePositions`)
    (bind _returnvalue (* _array_element SplineLength))
    (bind _returnvalue_2 (`AddComponent|NODE_AddChildActorComponent-2` :`RelativeTransform` (`KismetMathLibrary.MakeTransform` (`SplineComponent.GetLocationAtDistanceAlongSpline` Spline _returnvalue "Local") (`KismetMathLibrary.MakeRotFromX` (`SplineComponent.GetTangentAtDistanceAlongSpline` Spline _returnvalue "Local")))))
    (bind _asbp_valve (cast `/Game/Blueprints/Production/BP_Valve` (`ChildActorComponent.ChildActor` _returnvalue_2)))
    (`KismetArrayLibrary.Array_AddUnique` (`self.ValveReferences`) _asbp_valve))
  (for _array_element_2 (`self.ValveReferences`)
    (if (not (`/Game/Blueprints/Production/BP_Valve.IsOpen` _array_element_2))
      (set `self.IsFlowing` false)))
  (set `self.IsFlowing` true))

(fn `VolumeCalculationMain`
  (params (Tick :type "Float (double-precision)"))
  (bind _pump (`self.Pump`))
  (bind _source (`self.Source`))
  (bind _target (`self.Target`))
  (bind _fluidlevel (`/Game/Blueprints/Production/BP_Silo.FluidLevel` _source))
  (bind _returnvalue (* (`/Game/Blueprints/Production/BP_Pump.FlowRate` _pump) Tick))
  (bind _returnvalue_2 (- _fluidlevel _returnvalue))
  (set `self.IsFlowing` false)
  (if (`/Game/Blueprints/Production/BP_Pump.IsActive` _pump)
    (for _array_element (`self.ValveReferences`)
      (if (`/Game/Blueprints/Production/BP_Reactor.FinishedMixing` _target)
        (bind _isopen (`/Game/Blueprints/Production/BP_Valve.IsOpen` _array_element))
        (if _isopen
          (set `self.IsFlowing` true)
          (else
            (set `self.IsFlowing` false)
            (break)))
        (elif _isopen
          (`/Game/Blueprints/Production/BP_Valve.Interact` _array_element)
          (set `self.IsFlowing` false))))
    (if (`self.IsFlowing`)
      (if (< _returnvalue_2 0.0)
        (set `/Game/Blueprints/Production/BP_Silo.FluidLevel` 0.0 _source)
        (set `self.IsFlowing` false)
        (`self.UpdateFlowState`)
        (else
          (set `/Game/Blueprints/Production/BP_Silo.FluidLevel` _returnvalue_2 _source)
          (if (> (+ _returnvalue (`/Game/Blueprints/Production/BP_Reactor.FluidLevel` _target)) (`/Game/Blueprints/Production/BP_Reactor.MaxCapacity` _target))
            (set `self.IsFlowing` false)
            (`self.UpdateFlowState`)
            (else
              (set `self.MaterialAmount` _returnvalue)
              (`/Game/Blueprints/Production/BP_Reactor.UpdateFluidLevels` _target)))))
      (else
        (set `/Game/Blueprints/Production/BP_Silo.FluidLevel` (`KismetMathLibrary.Conv_IntToDouble` (* (`KismetMathLibrary.FFloor` (+ (/ _fluidlevel 100.0) 0.5)) 100)) _source)))))