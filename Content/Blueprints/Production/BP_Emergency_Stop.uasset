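; Emergency stop button for a production plant that shuts down the Educt A, Educt B and Product lines.
; Interact animates the button down, then TriggerES zeroes pumps, closes open valves, stops pipe flow and flags reactor mixing finished.
; Pump and flow states are saved in structs for RestoreAll, but valves are saved only as references, not open states.
; ResetES only animates the button, and RestoreAll leaves mixing untouched.
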(event `self.ReceiveBeginPlay`
  (set `self.InitialLocation` (`SceneComponent.RelativeLocation` (`self.EmergencyStopTop`))))

(event `TriggerES`
  (if (not (`self.IsTriggered`))
    (set `self.IsTriggered` true)
    (`self.ToggleAll`)))

(event `/Game/Blueprints/InteractionInterface.Interact`
  (if (not (`self.IsTriggered`))
    (bind (_direction _alpha) (`Timeline|Timeline`)
      (:`Update`
        (`SceneComponent.K2_SetRelativeLocation` (`self.EmergencyStopTop`) (+ (`KismetMathLibrary.MakeVector` 0.0 0.0 (* _alpha -1.0)) (`self.InitialLocation`)) false false))
      (:`Finished`
        (`self.TriggerES`)))))

(event `ResetES`
  (bind (_direction _alpha) (`Timeline|Timeline_0`)
    (:`Update`
      (`SceneComponent.K2_SetRelativeLocation` (`self.EmergencyStopTop`) (+ (`KismetMathLibrary.MakeVector` 0.0 0.0 _alpha) (`self.InitialLocation`)) false false))))

(fn `RestoreAll`
  (`self.RestoreEductA`)
  (`self.RestoreEductB`)
  (`self.RestoreProduct`)
  (set `self.IsTriggered` false))

(fn `RestoreEductA`
  (`self.RestorePumpEductA`)
  (`self.RestoreValvesEductA`))

(fn `RestoreEductB`
  (`self.RestorePumpEductB`)
  (`self.RestoreValvesEductB`))

(fn `RestoreProduct`
  (`self.RestorePumpProduct`)
  (`self.RestoreValvesProduct`))

(fn `RestorePumpEductA`
  (bind _pumpeducta (`self.PumpEductA`))
  (bind (_isactive _flowrate) (break `/Game/Blueprints/Production/FSTR_PumpState` (`self.PumpStructEductA`)))
  (set `/Game/Blueprints/Production/BP_Pump.IsActive` _isactive _pumpeducta)
  (set `/Game/Blueprints/Production/BP_Pump.FlowRate` _flowrate _pumpeducta))

(fn `RestorePumpEductB`
  (bind _pumpeductb (`self.PumpEductB`))
  (bind (_isactive _flowrate) (break `/Game/Blueprints/Production/FSTR_PumpState` (`self.PumpStructEductB`)))
  (set `/Game/Blueprints/Production/BP_Pump.IsActive` _isactive _pumpeductb)
  (set `/Game/Blueprints/Production/BP_Pump.FlowRate` _flowrate _pumpeductb))

(fn `RestorePumpProduct`
  (bind _pumpproduct (`self.PumpProduct`))
  (bind (_isactive _flowrate) (break `/Game/Blueprints/Production/FSTR_PumpState` (`self.PumpStructProduct`)))
  (set `/Game/Blueprints/Production/BP_Pump.IsActive` _isactive _pumpproduct)
  (set `/Game/Blueprints/Production/BP_Pump.FlowRate` _flowrate _pumpproduct))

(fn `RestoreValvesEductA`
  (bind _pipeeducta (`self.PipeEductA`))
  (bind (_valverefs _isflowing) (break `/Game/Blueprints/Production/FSTR_ValveState` (`self.ValveStructEductA`)))
  (for (_array_element _array_index) (`/Game/Blueprints/Production/Bp_pipe_straight_Silo_Reactor.ValveReferences` _pipeeducta)
    (if (!= (`/Game/Blueprints/Production/BP_Valve.IsOpen` (`|GetArrayItem` _valverefs _array_index)) (`/Game/Blueprints/Production/BP_Valve.IsOpen` _array_element))
      (`/Game/Blueprints/Production/BP_Valve.Interact` _array_element)))
  (set `/Game/Blueprints/Production/Bp_pipe_straight_Silo_Reactor.IsFlowing` _isflowing _pipeeducta))

(fn `RestoreValvesEductB`
  (bind _pipeeductb (`self.PipeEductB`))
  (bind (_valverefs _isflowing) (break `/Game/Blueprints/Production/FSTR_ValveState` (`self.ValveStructEductB`)))
  (for (_array_element _array_index) (`/Game/Blueprints/Production/Bp_pipe_straight_Silo_Reactor.ValveReferences` _pipeeductb)
    (if (!= (`/Game/Blueprints/Production/BP_Valve.IsOpen` _array_element) (`/Game/Blueprints/Production/BP_Valve.IsOpen` (`|GetArrayItem` _valverefs _array_index)))
      (`/Game/Blueprints/Production/BP_Valve.Interact` _array_element)))
  (set `/Game/Blueprints/Production/Bp_pipe_straight_Silo_Reactor.IsFlowing` _isflowing _pipeeductb))

(fn `RestoreValvesProduct`
  (bind _pipeproduct (`self.PipeProduct`))
  (bind (_valverefs _isflowing) (break `/Game/Blueprints/Production/FSTR_ValveState` (`self.ValveStructProduct`)))
  (for (_array_element _array_index) (`/Game/Blueprints/Production/Bp_pipe_straight_Reactor_Silo.ValveReferences` _pipeproduct)
    (if (!= (`/Game/Blueprints/Production/BP_Valve.IsOpen` _array_element) (`/Game/Blueprints/Production/BP_Valve.IsOpen` (`|GetArrayItem` _valverefs _array_index)))
      (`/Game/Blueprints/Production/BP_Valve.Interact` _array_element)))
  (set `/Game/Blueprints/Production/Bp_pipe_straight_Reactor_Silo.IsFlowing` _isflowing _pipeproduct))

(fn `ToggleAll`
  (`self.ToggleEductA`)
  (`self.ToggleEductB`)
  (`self.ToggleProduct`)
  (`self.ToggleMixing`))

(fn `ToggleEductA`
  (`self.TogglePumpEductA`)
  (`self.ToggleValvesEductA`))

(fn `ToggleEductB`
  (`self.TogglePumpEductB`)
  (`self.ToggleValvesEductB`))

(fn `ToggleMixing`
  (set `/Game/Blueprints/Production/BP_Reactor.FinishedMixing` true (`self.Reactor`)))

(fn `ToggleProduct`
  (`self.TogglePumpProduct`)
  (`self.ToggleValvesProduct`))

(fn `TogglePumpEductA`
  (bind _pumpeducta (`self.PumpEductA`))
  (set `self.PumpStructEductA` (make `/Game/Blueprints/Production/FSTR_PumpState` (`/Game/Blueprints/Production/BP_Pump.IsActive` _pumpeducta) (`/Game/Blueprints/Production/BP_Pump.FlowRate` _pumpeducta)))
  (set `/Game/Blueprints/Production/BP_Pump.IsActive` false _pumpeducta)
  (set `/Game/Blueprints/Production/BP_Pump.FlowRate` 0.0 _pumpeducta))

(fn `TogglePumpEductB`
  (bind _pumpeductb (`self.PumpEductB`))
  (set `self.PumpStructEductB` (make `/Game/Blueprints/Production/FSTR_PumpState` (`/Game/Blueprints/Production/BP_Pump.IsActive` _pumpeductb) (`/Game/Blueprints/Production/BP_Pump.FlowRate` _pumpeductb)))
  (set `/Game/Blueprints/Production/BP_Pump.IsActive` false _pumpeductb)
  (set `/Game/Blueprints/Production/BP_Pump.FlowRate` 0.0 _pumpeductb))

(fn `TogglePumpProduct`
  (bind _pumpproduct (`self.PumpProduct`))
  (set `self.PumpStructProduct` (make `/Game/Blueprints/Production/FSTR_PumpState` (`/Game/Blueprints/Production/BP_Pump.IsActive` _pumpproduct) (`/Game/Blueprints/Production/BP_Pump.FlowRate` _pumpproduct)))
  (set `/Game/Blueprints/Production/BP_Pump.IsActive` false _pumpproduct)
  (set `/Game/Blueprints/Production/BP_Pump.FlowRate` 0.0 _pumpproduct))

(fn `ToggleValvesEductA`
  (locals (NewLocalVar :type Boolean :default false))
  (bind _pipeeducta (`self.PipeEductA`))
  (bind _valvereferences (`/Game/Blueprints/Production/Bp_pipe_straight_Silo_Reactor.ValveReferences` _pipeeducta))
  (set `self.ValveStructEductA` (make `/Game/Blueprints/Production/FSTR_ValveState` _valvereferences (`/Game/Blueprints/Production/Bp_pipe_straight_Silo_Reactor.IsFlowing` _pipeeducta)))
  (for _array_element _valvereferences
    (if (`/Game/Blueprints/Production/BP_Valve.IsOpen` _array_element)
      (`/Game/Blueprints/Production/BP_Valve.Interact` _array_element)))
  (set `/Game/Blueprints/Production/Bp_pipe_straight_Silo_Reactor.IsFlowing` false _pipeeducta))

(fn `ToggleValvesEductB`
  (bind _pipeeductb (`self.PipeEductB`))
  (bind _valvereferences (`/Game/Blueprints/Production/Bp_pipe_straight_Silo_Reactor.ValveReferences` _pipeeductb))
  (set `self.ValveStructEductB` (make `/Game/Blueprints/Production/FSTR_ValveState` _valvereferences (`/Game/Blueprints/Production/Bp_pipe_straight_Silo_Reactor.IsFlowing` _pipeeductb)))
  (for _array_element _valvereferences
    (if (`/Game/Blueprints/Production/BP_Valve.IsOpen` _array_element)
      (`/Game/Blueprints/Production/BP_Valve.Interact` _array_element)))
  (set `/Game/Blueprints/Production/Bp_pipe_straight_Silo_Reactor.IsFlowing` false _pipeeductb))

(fn `ToggleValvesProduct`
  (bind _pipeproduct (`self.PipeProduct`))
  (bind _valvereferences (`/Game/Blueprints/Production/Bp_pipe_straight_Reactor_Silo.ValveReferences` _pipeproduct))
  (set `self.ValveStructProduct` (make `/Game/Blueprints/Production/FSTR_ValveState` _valvereferences (`/Game/Blueprints/Production/Bp_pipe_straight_Reactor_Silo.IsFlowing` _pipeproduct)))
  (for _array_element _valvereferences
    (if (`/Game/Blueprints/Production/BP_Valve.IsOpen` _array_element)
      (`/Game/Blueprints/Production/BP_Valve.Interact` _array_element)))
  (set `/Game/Blueprints/Production/Bp_pipe_straight_Reactor_Silo.IsFlowing` false _pipeproduct))

(fn `UserConstructionScript`
  (set `self.IsTriggered` false))