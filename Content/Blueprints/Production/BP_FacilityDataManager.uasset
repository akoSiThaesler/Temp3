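; Central data manager for a two-educt mixing facility, managing recipes, orders and equipment state.
; Every tick it mirrors silo, reactor, pump, pipe and emergency-stop values into its variables, with setters writing back to those actors.
; Starting an order validates volumes and an empty reactor, resets the three flow zones and begins filling Educt A; helpers switch to later stages.
; It also holds a day-night sun cycle that is not wired to run.
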(event `CreateRecipeFromInput`
  (params (Name :type Text) (EductA :type "Float (double-precision)") (EductB :type "Float (double-precision)") (MixingTime :type "Float (double-precision)"))
  (`self.CreateNewRecipe` Name EductA EductB MixingTime))

(event `GetRecipesByName`
  (params (Name :type Text))
  (`self.GetRecipe` Name))

(event `EditSingleRecipe`
  (params (Name :type Text) (EductA :type "Float (double-precision)") (EductB :type "Float (double-precision)") (MixingTime :type "Float (double-precision)") (NewName :type Text) (NewEductA :type "Float (double-precision)") (NewEductB :type "Float (double-precision)") (NewMixingTime :type "Float (double-precision)"))
  (`self.EditRecipe` Name EductA EductB MixingTime NewName NewEductA NewEductB NewMixingTime))

(event `DeleteSingleRecipe`
  (params (Name :type Text) (EductA :type "Float (double-precision)") (EductB :type "Float (double-precision)") (MixingTime :type "Float (double-precision)"))
  (`self.DeleteRecipe` Name EductA EductB MixingTime))

(event `CreateOrderFromInput`
  (params (SelectedRecipe :type "/Game/Blueprints/Production/STR_Recipe Structure"))
  (`self.CreateOrder` SelectedRecipe))

(event `GetOrderByID`
  (params (ID :type Integer))
  (`self.GetOrder` ID))

(event `StartOrder`
  (params (SelectedOrder :type "/Game/Blueprints/Production/STR_Order Structure"))
  (bind _canplaceorder (`self.CanExecuteOrder` SelectedOrder))
  (`self.SetOrderActive` _canplaceorder SelectedOrder)
  (if _canplaceorder
    (`self.DefaultProductionState`)
    (`self.ExecuteOrder` SelectedOrder)))

(event `DeleteOrder`
  (params (`Selected Order` :type "/Game/Blueprints/Production/STR_Order Structure"))
  (bind _activeorders (`self.ActiveOrders`))
  (for (_ _array_index) _activeorders
    (if (== _array_index (`.OrderID_12_45E7C4674765D1E8CC743E95390F45F6` (break `/Game/Blueprints/Production/STR_Order` `Selected Order`)))
      (`KismetArrayLibrary.Array_Remove` _activeorders _array_index)))
  (for (_array_element _array_index_2) _activeorders
    (bind _structout (setmembers `/Game/Blueprints/Production/STR_Order` :`StructRef` _array_element :`OrderID` _array_index_2))
    (`KismetArrayLibrary.Array_Set` _activeorders _array_index_2 _structout)))

(event `self.ReceiveTick`
  (params (DeltaSeconds :type "Float (single-precision)"))
  (`self.GetAllValues`))

(fn `CanExecuteOrder`
  (params (Order :type "/Game/Blueprints/Production/STR_Order Structure"))
  (returns (CanPlaceOrder :type Boolean))
  (bind (_recipename _amounteducta _amounteductb) (break `/Game/Blueprints/Production/STR_Recipe` (`.Recipe_2_D2B57C054B4D950C5B26099EBBD30DCD` (break `/Game/Blueprints/Production/STR_Order` Order))))
  (bind _returnvalue (+ _amounteducta _amounteductb))
  (if (<= _returnvalue (`self.MaxVolumeReactor`))
    (if (<= _returnvalue (- (`self.MaxVolumeSiloProduct`) (`self.FluidLevelSiloProduct`)))
      (if (<= _amounteducta (`self.FluidLevelSiloEductA`))
        (if (<= _amounteductb (`self.FluidLevelSiloEductB`))
          (if (== (`self.FluidLevelReactor`) 0.0)
            (set `self.OrderExecuteInfo` "Order Valid. Execution Starting. Monitor State via Fluid Level or Flow Information Screen")
            (return true)
            (else
              (set `self.OrderExecuteInfo` "Reactor not Empty at Current Stage. Wait until Emptying Process Finished")))
          (else
            (set `self.OrderExecuteInfo` "Ordered Amount Educt B Exceeds Available Amount")))
        (else
          (set `self.OrderExecuteInfo` "Ordered Amount Educt A Exceeds Available Amount")))
      (else
        (set `self.OrderExecuteInfo` "Product Amount Exceeds Product Silo Remaining Volume")))
    (else
      (set `self.OrderExecuteInfo` "Amount of Ordered Material Exceeds Reactor Max Volume")))
  (return false))

(fn `CreateNewRecipe`
  (params (Name :type Text) (EductA :type "Float (double-precision)") (EductB :type "Float (double-precision)") (MixingTime :type "Float (double-precision)"))
  (`self.RecipeExists` Name EductA EductB MixingTime)
  (if (`self.RecipeAlreadyExists`)
    (`KismetSystemLibrary.PrintText` "Recipe Already Exists!")
    (else
      (`KismetArrayLibrary.Array_Add` (`self.AvailableRecipes`) (make `/Game/Blueprints/Production/STR_Recipe` Name EductA EductB MixingTime (+ EductA EductB))))))

(fn `CreateOrder`
  (params (SelectedRecipe :type "/Game/Blueprints/Production/STR_Recipe Structure"))
  (bind _activeorders (`self.ActiveOrders`))
  (for (_array_element _array_index) _activeorders
    (bind _structout (setmembers `/Game/Blueprints/Production/STR_Order` :`StructRef` _array_element :`OrderID` _array_index))
    (`KismetArrayLibrary.Array_Set` _activeorders _array_index _structout))
  (`KismetArrayLibrary.Array_Add` _activeorders (make `/Game/Blueprints/Production/STR_Order` SelectedRecipe (`KismetMathLibrary.Now`) false (`KismetArrayLibrary.Array_Length` _activeorders))))

(fn `DayNightCycle`
  (params (Tick :type "Float (double-precision)"))
  (set `self.TimeOfDay` (mod (+ (* Tick (`self.DaySpeedMultiplier`) 60.0) (`self.TimeOfDay`)) 1440.0))
  (`self.SunRotation`)
  (`self.IsNightTest`))

(fn `DefaultProductionState`
  (`self.SetValveZone1` false)
  (`self.SetValveZone2` false)
  (`self.SetValveZone3` false)
  (`self.SetPumpZone1` true)
  (`self.SetPumpZone2` true)
  (`self.SetPumpZone3` true)
  (`self.SetFlowRateZone1` 10.0)
  (`self.SetFlowRateZone2` 10.0)
  (`self.SetFlowRateZone3` 10.0))

(fn `DeleteRecipe`
  (params (Name :type Text) (EductA :type "Float (double-precision)") (EductB :type "Float (double-precision)") (MixingTime :type "Float (double-precision)"))
  (bind _availablerecipes (`self.AvailableRecipes`))
  (for (_array_element _array_index) _availablerecipes
    (bind (_recipename _amounteducta _amounteductb _mixingtimeseconds) (break `/Game/Blueprints/Production/STR_Recipe` _array_element))
    (if (and (`KismetTextLibrary.EqualEqual_TextText` _recipename Name) (== _amounteducta EductA) (== _amounteductb EductB) (== _mixingtimeseconds MixingTime))
      (`KismetArrayLibrary.Array_Remove` _availablerecipes _array_index)
      (break))))

(fn `EditRecipe`
  (params (Name :type Text) (EductA :type "Float (double-precision)") (EductB :type "Float (double-precision)") (MixingTime :type "Float (double-precision)") (NewName :type Text) (NewEductA :type "Float (double-precision)") (NewEductB :type "Float (double-precision)") (NewMixingTime :type "Float (double-precision)"))
  (bind _availablerecipes (`self.AvailableRecipes`))
  (for (_array_element _array_index) _availablerecipes
    (bind (_recipename _amounteducta _amounteductb _mixingtimeseconds) (break `/Game/Blueprints/Production/STR_Recipe` _array_element))
    (if (and (`KismetTextLibrary.EqualEqual_TextText` _recipename Name) (== _amounteducta EductA) (== _amounteductb EductB) (== _mixingtimeseconds MixingTime))
      (`KismetArrayLibrary.Array_Set` _availablerecipes _array_index (make `/Game/Blueprints/Production/STR_Recipe` NewName NewEductA NewEductB NewMixingTime (+ NewEductA NewMixingTime)))
      (break))))

(fn `EmptyReactor`
  (`self.SetValveZone2` false)
  (`self.SetValveZone3` true))

(fn `ExecuteOrder`
  (params (Order :type "/Game/Blueprints/Production/STR_Order Structure"))
  (bind _reactor_ref (`self.Reactor_Ref`))
  (bind (_recipename _amounteducta _amounteductb _mixingtimeseconds) (break `/Game/Blueprints/Production/STR_Recipe` (`.Recipe_2_D2B57C054B4D950C5B26099EBBD30DCD` (break `/Game/Blueprints/Production/STR_Order` Order))))
  (set `/Game/Blueprints/Production/BP_Reactor.OrderedMaterialA` _amounteducta _reactor_ref)
  (set `/Game/Blueprints/Production/BP_Reactor.OrderedMaterialB` _amounteductb _reactor_ref)
  (set `/Game/Blueprints/Production/BP_Reactor.MixingDuration` _mixingtimeseconds _reactor_ref)
  (`self.FillEductA`))

(fn `FillEductA`
  (`self.SetValveZone1` true)
  (`self.SetPumpZone1` true)
  (`self.SetFlowRateZone1` 10.0))

(fn `FillEductB`
  (`self.SetValveZone1` false)
  (`self.SetValveZone2` true))

(fn `GetAllValues`
  (bind _siloeducta_ref (`self.SiloEductA_Ref`))
  (bind _siloeductb_ref (`self.SiloEductB_Ref`))
  (bind _siloproduct_ref (`self.SiloProduct_Ref`))
  (bind _pumpeducta_ref (`self.PumpEductA_Ref`))
  (bind _pumpeductb_ref (`self.PumpEductB_Ref`))
  (bind _pumpproduct_ref (`self.PumpProduct_Ref`))
  (bind _reactor_ref (`self.Reactor_Ref`))
  (set `self.FluidLevelSiloEductA` (`/Game/Blueprints/Production/BP_Silo.FluidLevel` _siloeducta_ref))
  (set `self.MaxVolumeSiloEductA` (`/Game/Blueprints/Production/BP_Silo.MaxCapacity` _siloeducta_ref))
  (set `self.TemperatureSiloEductA` (`/Game/Blueprints/Production/BP_Silo.Temperature` _siloeducta_ref))
  (set `self.FluidLevelSiloEductB` (`/Game/Blueprints/Production/BP_Silo.FluidLevel` _siloeductb_ref))
  (set `self.MaxVolumeSiloEductB` (`/Game/Blueprints/Production/BP_Silo.MaxCapacity` _siloeductb_ref))
  (set `self.TemperatureSiloEductB` (`/Game/Blueprints/Production/BP_Silo.Temperature` _siloeductb_ref))
  (set `self.FluidLevelSiloProduct` (`/Game/Blueprints/Production/BP_Silo.FluidLevel` _siloproduct_ref))
  (set `self.MaxVolumeSiloProduct` (`/Game/Blueprints/Production/BP_Silo.MaxCapacity` _siloproduct_ref))
  (set `self.TemperatureSiloProduct` (`/Game/Blueprints/Production/BP_Silo.Temperature` _siloproduct_ref))
  (set `self.FluidLevelReactor` (`/Game/Blueprints/Production/BP_Reactor.FluidLevel` _reactor_ref))
  (set `self.MaxVolumeReactor` (`/Game/Blueprints/Production/BP_Reactor.MaxCapacity` _reactor_ref))
  (set `self.TemperatureReactor` (`/Game/Blueprints/Production/BP_Reactor.Temperature` _reactor_ref))
  (set `self.FluidLevelReactorMatA` (`/Game/Blueprints/Production/BP_Reactor.MaterialA` _reactor_ref))
  (set `self.FluidLevelReactorMatB` (`/Game/Blueprints/Production/BP_Reactor.MaterialB` _reactor_ref))
  (set `self.VolumeOrderedReactorMatA` (`/Game/Blueprints/Production/BP_Reactor.OrderedMaterialA` _reactor_ref))
  (set `self.VolumeOrderedReactorMatB` (`/Game/Blueprints/Production/BP_Reactor.OrderedMaterialB` _reactor_ref))
  (set `self.MixingTimeLeft` (`/Game/Blueprints/Production/BP_Reactor.MixingTimeLeft` _reactor_ref))
  (set `self.IsMixing` (not (`/Game/Blueprints/Production/BP_Reactor.FinishedMixing` _reactor_ref)))
  (set `self.FlowRateZone1` (`/Game/Blueprints/Production/BP_Pump.FlowRate` _pumpeducta_ref))
  (set `self.ValvesZone1` (`/Game/Blueprints/Production/Bp_pipe_straight_Silo_Reactor.IsFlowing` (`self.PipeEductA_Ref`)))
  (set `self.PumpZone1` (`/Game/Blueprints/Production/BP_Pump.IsActive` _pumpeducta_ref))
  (set `self.FlowRateZone2` (`/Game/Blueprints/Production/BP_Pump.FlowRate` _pumpeductb_ref))
  (set `self.ValvesZone2` (`/Game/Blueprints/Production/Bp_pipe_straight_Silo_Reactor.IsFlowing` (`self.PipeEductB_Ref`)))
  (set `self.PumpZone2` (`/Game/Blueprints/Production/BP_Pump.IsActive` _pumpeductb_ref))
  (set `self.FlowRateZone3` (`/Game/Blueprints/Production/BP_Pump.FlowRate` _pumpproduct_ref))
  (set `self.ValvesZone3` (`/Game/Blueprints/Production/Bp_pipe_straight_Reactor_Silo.IsFlowing` (`self.PipeProduct_Ref`)))
  (set `self.PumpZone3` (`/Game/Blueprints/Production/BP_Pump.IsActive` _pumpproduct_ref))
  (set `self.SystemAlert` "")
  (set `self.EmergencyStopState` (`/Game/Blueprints/Production/BP_Emergency_Stop.IsTriggered` (`self.EmergencyStop`))))

(fn `GetOrder`
  (params (ID :type Integer))
  (returns (ActiveOrder :type "/Game/Blueprints/Production/STR_Order Structure") (Found :type Boolean))
  (for _array_element (`self.ActiveOrders`)
    (if (== ID (`.OrderID_12_45E7C4674765D1E8CC743E95390F45F6` (break `/Game/Blueprints/Production/STR_Order` _array_element)))
      (return _array_element true)))
  (return (struct) false))

(fn `GetRecipe`
  (params (RecipeName :type Text))
  (returns (Recipe :type "Array of /Game/Blueprints/Production/STR_Recipe Structure") (Found :type Boolean))
  (locals (TempRecipes :type "Array of /Game/Blueprints/Production/STR_Recipe Structure"))
  (bind _temprecipes (`local.TempRecipes`))
  (for _array_element (`self.AvailableRecipes`)
    (if (`KismetTextLibrary.EqualEqual_TextText` RecipeName (`.RecipeName_2_405A812F43A220AC194E28AF64AD6F3D` (break `/Game/Blueprints/Production/STR_Recipe` _array_element)))
      (`KismetArrayLibrary.Array_Add` _temprecipes _array_element)))
  (return _temprecipes (> (`KismetArrayLibrary.Array_Length` _temprecipes) 0)))

(fn `IsNightTest`
  (bind _timeofday (`self.TimeOfDay`))
  (if (or (>= _timeofday 1400.0) (< _timeofday 750.0))
    (set `self.IsNight?` true)
    (else
      (set `self.IsNight?` false))))

(fn `RecipeExists`
  (params (Name :type Text) (EductA :type "Float (double-precision)") (EductB :type "Float (double-precision)") (MixingTime :type "Float (double-precision)"))
  (set `self.RecipeAlreadyExists` false)
  (for _array_element (`self.AvailableRecipes`)
    (bind (_recipename _amounteducta _amounteductb _mixingtimeseconds) (break `/Game/Blueprints/Production/STR_Recipe` _array_element))
    (if (and (`KismetTextLibrary.EqualEqual_TextText` _recipename Name) (== _amounteducta EductA) (== _amounteductb EductB) (== _mixingtimeseconds MixingTime))
      (set `self.RecipeAlreadyExists` true)
      (break)
      (else
        (set `self.RecipeAlreadyExists` false)))))

(fn `SetFlowRateZone1`
  (params (FlowRate :type "Float (double-precision)"))
  (set `/Game/Blueprints/Production/BP_Pump.FlowRate` FlowRate (`self.PumpEductA_Ref`)))

(fn `SetFlowRateZone2`
  (params (FlowRate :type "Float (double-precision)"))
  (set `/Game/Blueprints/Production/BP_Pump.FlowRate` FlowRate (`self.PumpEductB_Ref`)))

(fn `SetFlowRateZone3`
  (params (FlowRate :type "Float (double-precision)"))
  (set `/Game/Blueprints/Production/BP_Pump.FlowRate` FlowRate (`self.PumpProduct_Ref`)))

(fn `SetFluidLevelReactor`
  (params (FluidLevel :type "Float (double-precision)"))
  (set `/Game/Blueprints/Production/BP_Reactor.FluidLevel` FluidLevel (`self.Reactor_Ref`)))

(fn `SetFluidLevelReactorMatA`
  (params (FluidLevelMatA :type "Float (double-precision)"))
  (set `/Game/Blueprints/Production/BP_Reactor.MaterialA` FluidLevelMatA (`self.Reactor_Ref`)))

(fn `SetFluidLevelReactorMatB`
  (params (FluidLevelMatB :type "Float (double-precision)"))
  (set `/Game/Blueprints/Production/BP_Reactor.MaterialB` FluidLevelMatB (`self.Reactor_Ref`)))

(fn `SetFluidLevelSiloEductA`
  (params (FluidLevel :type "Float (double-precision)"))
  (set `/Game/Blueprints/Production/BP_Silo.FluidLevel` FluidLevel (`self.SiloEductA_Ref`)))

(fn `SetFluidLevelSiloEductB`
  (params (FluidLevel :type "Float (double-precision)"))
  (set `/Game/Blueprints/Production/BP_Silo.FluidLevel` FluidLevel (`self.SiloEductB_Ref`)))

(fn `SetFluidLevelSiloProduct`
  (params (Volume :type "Float (double-precision)"))
  (set `/Game/Blueprints/Production/BP_Silo.FluidLevel` Volume (`self.SiloProduct_Ref`)))

(fn `SetMaxVolumeReactor`
  (params (Volume :type "Float (double-precision)"))
  (set `/Game/Blueprints/Production/BP_Reactor.MaxCapacity` Volume (`self.Reactor_Ref`)))

(fn `SetMaxVolumeSiloEductA`
  (params (Volume :type "Float (double-precision)"))
  (set `/Game/Blueprints/Production/BP_Silo.MaxCapacity` Volume (`self.SiloEductA_Ref`)))

(fn `SetMaxVolumeSiloEductB`
  (params (Volume :type "Float (double-precision)"))
  (set `/Game/Blueprints/Production/BP_Silo.MaxCapacity` Volume (`self.SiloEductB_Ref`)))

(fn `SetMaxVolumeSiloProduct`
  (params (Volume :type "Float (double-precision)"))
  (set `/Game/Blueprints/Production/BP_Silo.MaxCapacity` Volume (`self.SiloProduct_Ref`)))

(fn `SetOrderActive`
  (params (OrderState :type Boolean) (Order :type "/Game/Blueprints/Production/STR_Order Structure"))
  (bind _activeorders (`self.ActiveOrders`))
  (for (_array_element _array_index) _activeorders
    (if (== (`.OrderID_12_45E7C4674765D1E8CC743E95390F45F6` (break `/Game/Blueprints/Production/STR_Order` _array_element)) (`.OrderID_12_45E7C4674765D1E8CC743E95390F45F6` (break `/Game/Blueprints/Production/STR_Order` Order)))
      (bind _structout (setmembers `/Game/Blueprints/Production/STR_Order` :`StructRef` _array_element :`IsActive` OrderState))
      (`KismetArrayLibrary.Array_Set` _activeorders _array_index _structout))))

(fn `SetPumpZone1`
  (params (State :type Boolean))
  (set `/Game/Blueprints/Production/BP_Pump.IsActive` State (`self.PumpEductA_Ref`)))

(fn `SetPumpZone2`
  (params (State :type Boolean))
  (set `/Game/Blueprints/Production/BP_Pump.IsActive` State (`self.PumpEductB_Ref`)))

(fn `SetPumpZone3`
  (params (State :type Boolean))
  (set `/Game/Blueprints/Production/BP_Pump.IsActive` State (`self.PumpProduct_Ref`)))

(fn `SetSystemAlert`
  (params (SystemAlert :type Text))
  (set `self.SystemAlert` SystemAlert))

(fn `SetTemperatureReactor`
  (params (Temperature :type "Float (double-precision)"))
  (set `/Game/Blueprints/Production/BP_Reactor.Temperature` Temperature (`self.Reactor_Ref`)))

(fn `SetTemperatureSiloEductA`
  (params (Temperature :type "Float (double-precision)"))
  (set `/Game/Blueprints/Production/BP_Silo.Temperature` Temperature (`self.SiloEductA_Ref`)))

(fn `SetTemperatureSiloEductB`
  (params (Temperature :type "Float (double-precision)"))
  (set `/Game/Blueprints/Production/BP_Silo.Temperature` Temperature (`self.SiloEductB_Ref`)))

(fn `SetTemperatureSiloProduct`
  (params (Temperature :type "Float (double-precision)"))
  (set `/Game/Blueprints/Production/BP_Silo.Temperature` Temperature (`self.SiloProduct_Ref`)))

(fn `SetValveZone1`
  (params (State :type Boolean))
  (for _array_element (`/Game/Blueprints/Production/Bp_pipe_straight_Silo_Reactor.ValveReferences` (`self.PipeEductA_Ref`))
    (set `/Game/Blueprints/Production/BP_Valve.IsOpen` State _array_element)))

(fn `SetValveZone2`
  (params (State :type Boolean))
  (for _array_element (`/Game/Blueprints/Production/Bp_pipe_straight_Silo_Reactor.ValveReferences` (`self.PipeEductB_Ref`))
    (set `/Game/Blueprints/Production/BP_Valve.IsOpen` State _array_element)))

(fn `SetValveZone3`
  (params (State :type Boolean))
  (for _array_element (`/Game/Blueprints/Production/Bp_pipe_straight_Reactor_Silo.ValveReferences` (`self.PipeProduct_Ref`))
    (set `/Game/Blueprints/Production/BP_Valve.IsOpen` State _array_element)))

(fn `SetVolumeOrderedReactorMatA`
  (params (VolumeOrderedMatA :type "Float (double-precision)"))
  (set `/Game/Blueprints/Production/BP_Reactor.OrderedMaterialA` VolumeOrderedMatA (`self.Reactor_Ref`)))

(fn `SetVolumeOrderedReactorMatB`
  (params (VolumeOrderedMaterialB :type "Float (double-precision)"))
  (set `/Game/Blueprints/Production/BP_Reactor.OrderedMaterialB` VolumeOrderedMaterialB (`self.Reactor_Ref`)))

(fn `SunRotation`
  (`self.K2_SetActorRotation` (`self.SunLight`) (`KismetMathLibrary.MakeRotator` 0.0 (* (/ (`self.TimeOfDay`) 1440.0) 360.0)) false))

(fn `UserConstructionScript`
  (set `self.TimeOfDay` 1000.0)
  (set `self.IsNight?` false))