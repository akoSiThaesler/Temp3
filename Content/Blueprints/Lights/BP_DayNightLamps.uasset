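; Day/night lamp with a spot light and a point light that fade with the facility's night state.
; Tick polls IsNight on BP_FacilityDataManager and uses WasNight to act only on transitions.
; Nightfall activates both lights and shadows, then plays one intensity timeline per light; daybreak reverses them.
; The point light timeline's Finished event, not filtered by direction, deactivates both lights and their shadows.
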(event `self.ReceiveBeginPlay`
  (bind _outactors (`GameplayStatics.GetAllActorsOfClass` "/Game/Blueprints/Production/BP_FacilityDataManager.BP_FacilityDataManager_C"))
  (set `self.DataManager` (`|GetArrayItem` _outactors)))

(event `self.ReceiveTick`
  (params (DeltaSeconds :type "Float (single-precision)"))
  (bind _pointlight (`self.PointLight`))
  (bind _spotlight (`self.SpotLight`))
  (bind _wasnight_ (`self.wasNight?`))
  (if (`/Game/Blueprints/Production/BP_FacilityDataManager.IsNight?` (`self.Datamanager`))
    (if (not _wasnight_)
      (`ActorComponent.SetActive` _spotlight true false)
      (`LightComponentBase.SetCastShadows` _spotlight true)
      (`ActorComponent.SetActive` _pointlight true false)
      (`LightComponentBase.SetCastShadows` _pointlight true)
      (`|ExecutionSequence`
        (:`then_0`
          (bind (_direction _alpha) (`Timeline|Timeline` :!label _label)
            (:`Update`
              (`LightComponent.SetIntensity` _spotlight _alpha))))
        (:`then_1`
          (bind (_direction_2 _alpha_2) (`Timeline|Timeline_0` :!label _label_2)
            (:`Update`
              (`LightComponent.SetIntensity` _pointlight _alpha_2))
            (:`Finished`
              (`ActorComponent.SetActive` _spotlight false false)
              (`LightComponentBase.SetCastShadows` _spotlight false)
              (`ActorComponent.SetActive` _pointlight false false)
              (`LightComponentBase.SetCastShadows` _pointlight false))))
        (:`then_2`
          (set `self.wasNight?` true))))
    (elif _wasnight_
      (`|ExecutionSequence`
        (:`then_0`
          (goto _label :!via `Reverse`))
        (:`then_1`
          (goto _label_2 :!via `Reverse`))
        (:`then_2`
          (set `self.wasNight?` false))))))

(fn `UserConstructionScript`
  (`LightComponent.SetIntensity` (`self.SpotLight`) 0.0)
  (`LightComponent.SetIntensity` (`self.PointLight`) 0.0))